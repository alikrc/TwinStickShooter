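; Enemy character for a twin-stick game that damages the hero on contact and awards score when killed.
; Overlapping a HeroCharacter starts a looping damage timer paced by AttacksPerSecond, cleared when the overlap ends.
; Incoming damage updates and prints health; death increments the TwinStickMode score, disables capsule collision, detaches the controller and destroys the actor after a delay.
; The construction script tints the body through a dynamic material using EnemyColor.
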(event `DamageTheHero`
  ;[1 1 1] If Hit To Hero
  ;;[1 1 1] Damage The Hero
  (`GameplayStatics.ApplyDamage` (`self.Hero`) (`self.DamageToHero`) null self))

(event `self.ReceiveActorBeginOverlap`
  (params (OtherActor :type "Actor Object Reference"))
  ;[1 1 1] If Hit To Hero
  (bind _ashero_character (cast `/Game/Blueprints/HeroCharacter` OtherActor))
  (set `self.Hero` _ashero_character)
  (`KismetSystemLibrary.K2_SetTimerDelegate` (delegate `DamageTheHero`) (/ 1.0 (`self.AttacksPerSecond`)) true))

(event `self.ReceiveActorEndOverlap`
  (params (OtherActor :type "Actor Object Reference"))
  ;[1 1 1] STOP damage hero
  ;;[1 1 1] if ishero
  (if (== OtherActor (`self.Hero`))
    (`KismetSystemLibrary.K2_ClearTimer` null "DamageTheHero")))

(event `self.ReceiveAnyDamage`
  (params (Damage :type "Float (single-precision)") (DamageType :type "DamageType Object Reference") (InstigatedBy :type "Controller Object Reference") (DamageCauser :type "Actor Object Reference"))
  (`self.CalculateHealth` Damage)
  (`KismetSystemLibrary.PrintString` (`KismetStringLibrary.Conv_DoubleToString` (`self.Health`)) true true (struct :`R` 0.953125 :`G` 0.87272 :`B` 0.86322 :`A` 1.0) 3.0)
  (if (`self.isDead`)
    ;[1 1 1] set score
    (bind _astwin_stick_mode (cast `/Game/Blueprints/TwinStickMode` (`GameplayStatics.GetGameMode`)))
    (`/Game/Blueprints/TwinStickMode.IncrementScore` _astwin_stick_mode (`self.GainedScore`))
    ;[1 1 1] dying anim
    (`PrimitiveComponent.SetCollisionResponseToAllChannels` (`self.CapsuleComponent`) "ECR_Ignore")
    (`self.DetachFromControllerPendingDestroy`)
    (`KismetSystemLibrary.Delay` 3.0)
    (`self.K2_DestroyActor`)))

(fn `UserConstructionScript`
  (bind _returnvalue (`PrimitiveComponent.CreateDynamicMaterialInstance` (`self.Mesh`) 0 null "None"))
  (bind _output_get (set `self.DynoMat` _returnvalue))
  (`MaterialInstanceDynamic.SetVectorParameterValue` _output_get "BodyColor" (`self.EnemyColor`)))